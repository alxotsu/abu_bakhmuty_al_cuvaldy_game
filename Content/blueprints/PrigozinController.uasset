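; PrigozinController is a player controller that makes the possessed pawn follow the mouse cursor on a fixed plane.
; Each tick it line traces 2000 units from the deprojected cursor and sweeps the pawn's root to the hit's X and Z, with Y pinned to 1.
; Its PawnHit function forwards the hit object and itself to PrigozinGameMode, which handles the hit.
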(event `self.ReceiveTick`
  (params (DeltaSeconds :type "Float (single-precision)"))
  (bind (_worldlocation _worlddirection) (`self.DeprojectMousePositionToWorld` self))
  (bind _outhit (`KismetSystemLibrary.LineTraceSingle` _worldlocation (+ _worldlocation (* _worlddirection 2000.0)) "TraceTypeQuery1"))
  (`SceneComponent.K2_SetWorldLocation` (`Actor.RootComponent` (`self.K2_GetPawn` self)) (`KismetMathLibrary.MakeVector` (.x (`.Location` (`GameplayStatics.BreakHitResult` _outhit))) 1.0 (.z (`.Location` (`GameplayStatics.BreakHitResult` _outhit)))) true false))

(fn `PawnHit`
  (params (HittedObj :type "Actor Object Reference"))
  (bind _asgame_mode (cast `/Game/blueprints/PrigozinGameMode` (`GameplayStatics.GetGameMode`)))
  (`/Game/blueprints/PrigozinGameMode.Pawn Hit Object` _asgame_mode HittedObj self))

(fn `UserConstructionScript`)