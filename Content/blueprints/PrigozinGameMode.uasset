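; PrigozinGameMode runs a catch-the-falling-objects game, handling both object spawning and scoring.
; From BeginPlay, an endless delay loop spawns a random FallObjectClasses entry every half second at height, with random horizontal position, pitch and scale.
; PawnHitObject adds a point for BaseBoepripas hits and resets the score for BaseGilza hits.
; Both hit types push the score to the player's HUD and destroy the object.
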(event `self.ReceiveBeginPlay`
  (bind _returnvalue (`KismetMathLibrary.RandomFloatInRange` 0.7 1.5))
  (`KismetSystemLibrary.Delay` 0.5 :!label _label)
  (bind _result (`BlueprintSetLibrary.Set_ToArray` (`self.FallObjectClasses`)))
  (`|SpawnActorFromClass` (`KismetArrayLibrary.Array_Random` _result) (`KismetMathLibrary.MakeTransform` (`KismetMathLibrary.MakeVector` (`KismetMathLibrary.RandomFloatInRange` -800.0 800.0) 1.0 800.0) (`KismetMathLibrary.MakeRotator` 0.0 (`KismetMathLibrary.RandomFloatInRange` -180.0 180.0)) (`KismetMathLibrary.MakeVector` _returnvalue _returnvalue _returnvalue)) "Undefined" "MultiplyWithRoot" null null)
  (goto _label))

(fn `Pawn Hit Object`
  (params (`Hitted Obj` :type "Actor Object Reference") (Player :type "/Game/blueprints/PrigozinController Object Reference"))
  (bind _ashud (cast `/Game/blueprints/HUD` (`PlayerController.GetHUD` Player)))
  (cast `/Game/blueprints/objects/BaseBoepripas` `Hitted Obj`
    (:`then`
      (set `self.Scores` (+ (`self.Scores`) 1)))
    (:`CastFailed`
      (cast `/Game/blueprints/objects/BaseGilza` `Hitted Obj`)
      (set `self.Scores` 0)))
  (`/Game/blueprints/HUD.Set Score` _ashud (`self.Scores`))
  (`self.K2_DestroyActor` `Hitted Obj`))

(fn `UserConstructionScript`)