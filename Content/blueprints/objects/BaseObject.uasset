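; BaseObject is a falling object whose RenderComponent moves straight down in world Z every frame.
; BeginPlay casts the game mode to PrigozinGameMode and caches its ObjectFallSpeed as FallSpeed.
; Tick subtracts FallSpeed from the component's Z with a swept SetWorldLocation.
; The step is not scaled by delta time, so fall speed depends on frame rate.
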(event `self.ReceiveBeginPlay`
  (bind _asprigozin_game_mode (cast `/Game/blueprints/PrigozinGameMode` (`GameplayStatics.GetGameMode`)))
  (set `self.fallSpeed` (`/Game/blueprints/PrigozinGameMode.ObjectFallSpeed` _asprigozin_game_mode)))

(event `self.ReceiveTick`
  (params (DeltaSeconds :type "Float (single-precision)"))
  (bind _rendercomponent (`self.RenderComponent`))
  (`SceneComponent.K2_SetWorldLocation` _rendercomponent (`KismetMathLibrary.MakeVector` (.x (`SceneComponent.K2_GetComponentLocation` _rendercomponent)) (.y (`SceneComponent.K2_GetComponentLocation` _rendercomponent)) (- (.z (`SceneComponent.K2_GetComponentLocation` _rendercomponent)) (`self.fallSpeed`))) true false))

(fn `UserConstructionScript`)