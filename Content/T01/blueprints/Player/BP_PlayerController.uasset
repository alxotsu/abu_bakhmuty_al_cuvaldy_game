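; BP_PlayerController is the player controller that moves the controlled pawn, toggles pause and reports pawn collisions.
; Up and right axis inputs feed MovePawn, which offsets the pawn's root on the X/Z plane with a swept SetWorldLocation, without delta-time scaling.
; The Pause action flips BP_PlayerState between two enum states.
; PawnHit forwards the hit object and this controller to BP_GameMode's PawnHitObject.
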(event `InputAxis|moveUp`
  (params (AxisValue :type "Float (single-precision)"))
  (`self.MovePawn` 0.0 AxisValue))

(event `InputAxis|moveRight`
  (params (AxisValue :type "Float (single-precision)"))
  (`self.MovePawn` AxisValue))

(event `InputAction|Pause`
  (params (Key :type "Key Structure"))
  (:`Pressed`
    (bind _asbp_player_state (cast `/Game/T01/blueprints/Player/BP_PlayerState` (`self.PlayerState`)))
    (bind _playerstate (`/Game/T01/blueprints/Player/BP_PlayerState.PlayerState` _asbp_player_state))
    (if (`|EnumEquality` _playerstate "NewEnumerator0")
      (`/Game/T01/blueprints/Player/BP_PlayerState.SetState` _asbp_player_state "NewEnumerator1")
      (elif (`|EnumEquality` _playerstate "NewEnumerator1")
        (`/Game/T01/blueprints/Player/BP_PlayerState.SetState` _asbp_player_state "NewEnumerator0")))))

(event `MovePawn`
  (params (X :type "Float (double-precision)") (Z :type "Float (double-precision)"))
  (bind _rootcomponent (`Actor.RootComponent` (`self.K2_GetPawn` self)))
  (`SceneComponent.K2_SetWorldLocation` _rootcomponent (`KismetMathLibrary.MakeVector` (+ X (.x (`SceneComponent.K2_GetComponentLocation` _rootcomponent))) (.y (`SceneComponent.K2_GetComponentLocation` _rootcomponent)) (+ (.z (`SceneComponent.K2_GetComponentLocation` _rootcomponent)) Z)) true false))

(fn `PawnHit`
  (params (HittedObj :type "Actor Object Reference"))
  (bind _asbp_game_mode (cast `/Game/T01/blueprints/Game/BP_GameMode` (`GameplayStatics.GetGameMode`)))
  (`/Game/T01/blueprints/Game/BP_GameMode.Pawn Hit Object` _asbp_game_mode HittedObj self))

(fn `UserConstructionScript`)