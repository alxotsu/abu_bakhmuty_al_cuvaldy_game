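; BP_PlayerState tracks the player's score and game state and pushes both to the HUD.
; SetScore stores the score and forwards it to BP_HUD.
; SetState stores the state, unpauses the game for Play and pauses it for Pause, End Game and Game Win, then passes the state to BP_HUD.
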(fn `SetScore`
  (params (Score :type Integer))
  (returns (_ :type Integer))
  (bind _output_get (set `self.PlayerScore` Score))
  (bind _asbp_hud (cast `/Game/T01/blueprints/Player/UI/BP_HUD` (`PlayerController.GetHUD` (`self.GetPlayerController`))))
  (`/Game/T01/blueprints/Player/UI/BP_HUD.Set Score` _asbp_hud _output_get)
  (return _output_get))

(fn `SetState`
  (params (State :type "/Game/T01/blueprints/Player/EPlayerState Enum" :default "NewEnumerator0"))
  (bind _output_get (set `self.PlayerState` State))
  (switch `/Game/T01/blueprints/Player/EPlayerState` _output_get
    (:`NewEnumerator0`
      (`GameplayStatics.SetGamePaused` false))
    (:`NewEnumerator1`
      (`GameplayStatics.SetGamePaused` true :!label _label))
    (:`NewEnumerator2`
      (goto _label))
    (:`NewEnumerator3`
      (goto _label)))
  (bind _asbp_hud (cast `/Game/T01/blueprints/Player/UI/BP_HUD` (`PlayerController.GetHUD` (`self.GetPlayerController`))))
  (`/Game/T01/blueprints/Player/UI/BP_HUD.SetState` _asbp_hud (`self.PlayerState`)))

(fn `UserConstructionScript`)