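; BP_GameMode runs a falling-object catching game, spawning objects and handling scoring, player state and restarts.
; A looping timer spawns a random FallObjectClasses actor at random horizontal position, pitch and scale.
; PawnHitObject scores and destroys BP_BaseBoepripas hits, raising ObjectFallSpeed with score, while BP_BaseGilza hits switch the BP_PlayerState state.
; NewGame resets speed, score and state, and destroys the actors in SpawnedObjects.
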(event `self.ReceiveBeginPlay`
  (bind _returnvalue (`KismetSystemLibrary.K2_SetTimerDelegate` (delegate `SpawnObject`) 0.5 true 2.0))
  (setmembers `TimerHandle` :`StructRef` _returnvalue))

(event `SpawnObject`
  (bind _returnvalue (`KismetMathLibrary.RandomFloatInRange` 0.7 1.5))
  (bind _result (`BlueprintSetLibrary.Set_ToArray` (`self.FallObjectClasses`)))
  (`|SpawnActorFromClass` (`KismetArrayLibrary.Array_Random` _result) (`KismetMathLibrary.MakeTransform` (`KismetMathLibrary.MakeVector` (`KismetMathLibrary.RandomFloatInRange` -800.0 800.0) 1.0 800.0) (`KismetMathLibrary.MakeRotator` 0.0 (`KismetMathLibrary.RandomFloatInRange` -180.0 180.0)) (`KismetMathLibrary.MakeVector` _returnvalue _returnvalue _returnvalue)) "Undefined" "MultiplyWithRoot" null null))

(fn `New Game`
  (params (Player :type "/Game/T01/blueprints/Player/BP_PlayerController Object Reference"))
  (set `self.ObjectFallSpeed` 1.0)
  (bind _asbp_player_state (cast `/Game/T01/blueprints/Player/BP_PlayerState` (`Controller.PlayerState` Player)))
  (bind _result (`BlueprintSetLibrary.Set_ToArray` (`self.SpawnedObjects`)))
  (for _array_element _result
    (`self.K2_DestroyActor` _array_element))
  (`/Game/T01/blueprints/Player/BP_PlayerState.SetState` _asbp_player_state "NewEnumerator0")
  (`/Game/T01/blueprints/Player/BP_PlayerState.SetScore` _asbp_player_state 0))

(fn `Pawn Hit Object`
  (params (`Hitted Obj` :type "Actor Object Reference") (Player :type "/Game/T01/blueprints/Player/BP_PlayerController Object Reference"))
  (bind _asbp_player_state (cast `/Game/T01/blueprints/Player/BP_PlayerState` (`Controller.PlayerState` Player)))
  (cast `/Game/T01/blueprints/Objects/BP_BaseBoepripas` `Hitted Obj`
    (:`then`
      (bind __ (`/Game/T01/blueprints/Player/BP_PlayerState.SetScore` _asbp_player_state (+ (`/Game/T01/blueprints/Player/BP_PlayerState.PlayerScore` _asbp_player_state) 1)))
      (`self.K2_DestroyActor` `Hitted Obj`)
      (set `self.ObjectFallSpeed` (+ (/ (`KismetMathLibrary.Conv_IntToDouble` __) 50.0) 1.0)))
    (:`CastFailed`
      (cast `/Game/T01/blueprints/Objects/BP_BaseGilza` `Hitted Obj`)
      (`/Game/T01/blueprints/Player/BP_PlayerState.SetState` _asbp_player_state "NewEnumerator2"))))

(fn `UserConstructionScript`)